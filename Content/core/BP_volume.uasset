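; BP_volume is an actor with a sphere volume that pushes physics objects upward while they are inside it.
; Sphere begin and end overlap events add and remove actors from an array.
; Every tick it loops over that array, casts each actor's root to a primitive component and applies a constant upward force as an acceleration change, so mass has no effect.
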(event OnComponentBeginOverlap(Sphere)
  (params (OverlappedComponent :type Primitive%20Component%20Object%20Reference) (OtherActor :type Actor%20Object%20Reference) (OtherComp :type Primitive%20Component%20Object%20Reference) (OtherBodyIndex :type Integer) (bFromSweep :type Boolean) (SweepResult :type Hit%20Result%20Structure%20%28by%20ref%29))
  (Utilities|Array|Add (Variables|Default|GetOther%20Actor) OtherActor))

(event OnComponentEndOverlap(Sphere)
  (params (OverlappedComponent :type Primitive%20Component%20Object%20Reference) (OtherActor :type Actor%20Object%20Reference) (OtherComp :type Primitive%20Component%20Object%20Reference) (OtherBodyIndex :type Integer))
  (Utilities|Array|RemoveItem (Variables|Default|GetOther%20Actor) OtherActor))

(event EventTick
  (params (DeltaSeconds :type Float%20%28single-precision%29))
  (for _array_element (Variables|Default|GetOther%20Actor)
    (bind _asprimitive_component (Utilities|Casting|CastToPrimitiveComponent (Variables|/Script/Engine.Actor|GetRootComponent _array_element)))
    (Physics|AddForce _asprimitive_component "0, 0,2000.000000" "None" true)))

(fn ConstructionScript)