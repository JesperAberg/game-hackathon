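; BP_cannon is an actor that fires BP_cannonBall projectiles continuously from BeginPlay.
; A self-looping Sequence and Delay spawns a ball at the Scene component's location every tenth of a second.
; Each ball's Sphere gets a physics velocity along the Cylinder's up vector scaled by LaunchSpeed, plus a random vector that grows with game time, so the spread steadily widens.
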(event EventBeginPlay
  (Utilities|FlowControl|Sequence :!label _label
    (:then_0
      (bind _returnvalue (Game|SpawnActorfromClass "/Game/core/BP_cannonBall.BP_cannonBall_C" (Math|Transform|MakeTransform (.location (Transformation|GetWorldTransform (Variables|Default|GetScene))) "0, 0, 0" "1.000000,1.000000,1.000000") "Undefined" self 0))
      (Physics|SetPhysicsLinearVelocity (Variables|/Game/core/BP_cannonBall.BP_cannonBall_C|GetSphere _returnvalue) (+ (* (Math|Vector|GetUpVector (Variables|Default|GetCylinder)) (Variables|Default|GetlaunchSpeed)) (* (Math|Random|RandomUnitVector) (* (Math|Float|MakeLiteralFloat 1e+02) (Utilities|Time|GetGameTimeinSeconds)))) false "None"))
    (:then_1
      (Utilities|FlowControl|Delay 0.1)
      (goto _label))))

(fn ConstructionScript)