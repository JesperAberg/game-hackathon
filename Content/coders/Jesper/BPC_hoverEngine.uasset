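; Hover engine scene component that pushes a physics Chassi away from surfaces beneath it, acting as a raycast spring-damper.
; Each tick it traces along its local down axis for world static and dynamic objects, ignoring its owner.
; On a hit it applies compression-scaled spring force plus velocity damping at its location, with separate compressing and relaxing dampers.
; BeginPlay also sets global time dilation to half speed.
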(event EventTick
  (params (DeltaSeconds :type Float%20%28single-precision%29))
  (bind _returnvalue (Transformation|GetWorldLocation))
  (bind (_outhit _returnvalue_2) (Collision|LineTraceForObjects _returnvalue (+ _returnvalue (* (Math|Vector|NegateVector (Math|Vector|GetUpVector (Transformation|GetWorldRotation))) (Variables|specs|GettraceDistance))) (Utilities|Array|MakeArray "ObjectTypeQuery1" "ObjectTypeQuery2") false (Utilities|Array|MakeArray (Components|GetOwner)) "None"))
  (if _returnvalue_2
    (bind _chassi (Variables|Default|Getchassi)
      (:then
        (bind _returnvalue_3 (Class|PrimitiveComponent|GetPhysicsLinearVelocityatPoint (Variables|Default|Getchassi) (Transformation|GetWorldLocation) "None"))
        (Class|PrimitiveComponent|AddForceatLocation _chassi (+ (* (Math|Float|SelectFloat (Variables|Specs|GetcompressingDamper) (* (Variables|Specs|GetrelaxingDamper) -1.0) (> (Math|Vector|DotProduct (Math|Vector|ProjectVectorontoVector _returnvalue_3 (Math|Vector|GetUpVector)) (Math|Vector|NegateVector (Math|Vector|GetUpVector))) 0.0)) (Math|Vector|VectorLength (Math|Vector|ProjectVectorontoVector _returnvalue_3 (Math|Vector|GetUpVector))) (Math|Vector|GetUpVector)) (* (Math|Vector|GetUpVector) (Variables|specs|Getforce) (- (Variables|specs|GettraceDistance) (.Distance (Collision|BreakHitResult _outhit))))) (Transformation|GetWorldLocation) "None"))
      (:else))))

(event EventBeginPlay
  (Utilities|Time|SetGlobalTimeDilation 0.5))