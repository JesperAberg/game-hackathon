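; A physics-driven hovering robot pawn that the first player controller possesses at BeginPlay.
; Each tick, the MoveForward and MoveRight inputs apply forward force and yaw torque to the Chassi body.
; The construction script hands Chassi to four hover engine components.
; Each Space Bar press permanently increases every engine's trace distance by a fixed step.
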(event EventBeginPlay
  (Pawn|Possess (Game|GetPlayerController 0) self))

(event EventTick
  (params (DeltaSeconds :type Float%20%28single-precision%29))
  (Physics|AddForce (Variables|Default|Getchassi) (* (Transformation|GetActorForwardVector) (Input|AxisValues|GetmoveForward) (Math|Float|MakeLiteralFloat 1e+05)) "None" false)
  (Class|PrimitiveComponent|AddTorqueinRadians (Variables|Default|Getchassi) (* (Transformation|GetActorUpVector) (Input|AxisValues|GetmoveRight) (Math|Float|MakeLiteralFloat 3e+05)) "None" false))

(event Input|KeyboardEvents|SpaceBar
  (params (Key :type Key%20Structure :default "None"))
  (:Pressed
    (for _array_element (Utilities|Array|MakeArray (Variables|Default|GetBPC_hoverEngine1) (Variables|Default|GetBPC_hoverEngine2) (Variables|Default|GetBPC_hoverEngine3) (Variables|Default|GetBPC_hoverEngine))
      (Variables|/Game/coders/Jesper/BPC_hoverEngine.BPC_hoverEngine_C|SettraceDistance _array_element (+ (Variables|/Game/coders/Jesper/BPC_hoverEngine.BPC_hoverEngine_C|GettraceDistance _array_element) 1e+01)))))

(fn ConstructionScript
  (Variables|/Game/coders/Jesper/BPC_hoverEngine.BPC_hoverEngine_C|Setchassi (Variables|Default|GetBPC_hoverEngine1) (Variables|Default|Getchassi))
  (Variables|/Game/coders/Jesper/BPC_hoverEngine.BPC_hoverEngine_C|Setchassi (Variables|Default|GetBPC_hoverEngine2) (Variables|Default|Getchassi))
  (Variables|/Game/coders/Jesper/BPC_hoverEngine.BPC_hoverEngine_C|Setchassi (Variables|Default|GetBPC_hoverEngine3) (Variables|Default|Getchassi))
  (Variables|/Game/coders/Jesper/BPC_hoverEngine.BPC_hoverEngine_C|Setchassi (Variables|Default|GetBPC_hoverEngine) (Variables|Default|Getchassi)))