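; BP_LaunchPad is a launch pad actor that fires at random intervals by swinging its Cylinder.
; A delayed Tick rolls a 50% chance about once per second, with a gate enforcing a short cooldown after firing.
; On firing, a sphere overlap around the Cube wakes rigid bodies on nearby dynamic actors, then a timeline drives the Cylinder's relative rotation, presumably to fling them.
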(event EventBeginPlay)

(event Collision|EventActorBeginOverlap
  (params (OtherActor :type Actor%20Object%20Reference)))

(event EventTick
  (params (DeltaSeconds :type Float%20%28single-precision%29))
  (bind _cube (Variables|Default|GetCube))
  (Utilities|FlowControl|Delay 1.0)
  (if (> 0.5 (Math|Random|RandomFloat))
    (Utilities|FlowControl|Sequence
      (:then_0
        (Utilities|FlowControl|Gate false :!label _label
          (:Exit
            (bind _outactors (Collision|SphereOverlapActors (Transformation|GetWorldLocation _cube) (.SphereRadius (Collision|GetComponentBounds _cube)) (Utilities|Array|MakeArray "ObjectTypeQuery2") "/Script/Engine.Actor"))
            (for _array_element _outactors
              (bind _asprimitive_component (Utilities|Casting|CastToPrimitiveComponent (Variables|/Script/Engine.Actor|GetRootComponent _array_element)))
              (Class|PrimitiveComponent|WakeAllRigidBodies _asprimitive_component))
            (bind _newtrack_0 (Timeline|Interpolation Play)
              (:Update
                (Transformation|SetRelativeRotation (Variables|Default|GetCylinder) (Math|Rotator|MakeRotator 0.0 0.0 (* _newtrack_0 -75.0)) false false))))))
      (:then_1
        (goto _label Close))
      (:then_2
        (Utilities|FlowControl|Delay 3.0)
        (goto _label Open)))))

(fn ConstructionScript)